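; Player controller that handles first-person style input for movement, looking, shooting and jumping on the local player's pawn.
; BeginPlay adds the IMC_Player Enhanced Input mapping context, and each input action drives player index 0's pawn or character directly.
; Movement follows the pawn's right and forward vectors, look pitch is inverted, and shooting is sent to the pawn as a Shoot message call.
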(event `self.ReceiveBeginPlay`
  ;[1 1 1] Enable Inputs
  (`EnhancedInputSubsystemInterface.AddMappingContext` (subsystem `EnhancedInputLocalPlayerSubsystem`) "/Game/Input/IMC_Player.IMC_Player" 0 (struct)))

(event `EnhancedInput|/Game/Input/Actions/IA_Move`
  (params (ActionValue :type "Vector2D Structure") (ElapsedSeconds :type "Float (double-precision)") (TriggeredSeconds :type "Float (double-precision)") (InputAction :type "InputAction Object Reference" :default "/Game/Input/Actions/IA_Move.IA_Move"))
  (bind _returnvalue (`GameplayStatics.GetPlayerPawn` 0))
  (bind (_x _y) (`KismetMathLibrary.BreakVector2D` ActionValue))
  ;[1 1 1] Movement
  (:`Triggered`
    (`Pawn.AddMovementInput` _returnvalue (`self.GetActorRightVector` _returnvalue) _x false)
    (`Pawn.AddMovementInput` _returnvalue (`self.GetActorForwardVector` _returnvalue) _y false)))

(event `EnhancedInput|/Game/Input/Actions/IA_Look`
  (params (ActionValue :type "Vector2D Structure") (ElapsedSeconds :type "Float (double-precision)") (TriggeredSeconds :type "Float (double-precision)") (InputAction :type "InputAction Object Reference" :default "/Game/Input/Actions/IA_Look.IA_Look"))
  (bind _returnvalue (`GameplayStatics.GetPlayerPawn` 0))
  (bind (_x _y) (`KismetMathLibrary.BreakVector2D` ActionValue))
  ;[1 1 1] Looking around
  (:`Triggered`
    (`Pawn.AddControllerYawInput` _returnvalue _x)
    (`Pawn.AddControllerPitchInput` _returnvalue (* _y -1.0))))

(event `EnhancedInput|/Game/Input/Actions/IA_Shoot`
  (params (ActionValue :type Boolean) (ElapsedSeconds :type "Float (double-precision)") (TriggeredSeconds :type "Float (double-precision)") (InputAction :type "InputAction Object Reference" :default "/Game/Input/Actions/IA_Shoot.IA_Shoot"))
  ;[1 1 1] Shooting
  (:`Triggered`
    (message `/Game/Blueprints/Interfaces/BPI_Player.Shoot` (`GameplayStatics.GetPlayerPawn` 0))))

(event `EnhancedInput|/Game/Input/Actions/IA_Jump`
  (params (ActionValue :type Boolean) (ElapsedSeconds :type "Float (double-precision)") (TriggeredSeconds :type "Float (double-precision)") (InputAction :type "InputAction Object Reference" :default "/Game/Input/Actions/IA_Jump.IA_Jump"))
  (bind _returnvalue (`GameplayStatics.GetPlayerCharacter` 0))
  ;[1 1 1] Jumping
  (:`Triggered`
    (`Character.Jump` _returnvalue))
  (:`Canceled`
    (`Character.StopJumping` _returnvalue)))

(fn `UserConstructionScript`)