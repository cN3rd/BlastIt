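; BP_Player is the player character, handling weapons, sprinting and a detection risk meter that can fail the game.
; Equipping snaps a weapon to GunPosition with physics off, while unequipping detaches it with physics on, and shooting forwards to the current weapon.
; Tick broadcasts risk changes and raises or lowers Risk over ten seconds based on the at-risk flag, triggering BP_GameMode's failed game over when full.
; Hit is an empty stub.
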(event `/Game/Blueprints/Interfaces/BPI_Player.EquipWeapon`
  (params (`New Weapon` :type "/Game/Blueprints/Weapons/BP_WeaponBase Object Reference"))
  (`/Game/Blueprints/Interfaces/BPI_PickableWeapon.Set Weapon Physics Simulation` `New Weapon` false)
  (`self.K2_AttachToComponent` `New Weapon` (`self.Gun Position`) "None" "SnapToTarget" "SnapToTarget" "KeepRelative" true)
  (set `self.CurrentWeapon` `New Weapon`)
  (`self.OnEquipWeapon`))

(event `/Game/Blueprints/Interfaces/BPI_Player.Shoot`
  (bind _currentweapon (`self.CurrentWeapon`))
  (`/Engine/EditorBlueprintResources/StandardMacros.IsValid` _currentweapon
    (:`Is Valid`
      (message `/Game/Blueprints/Interfaces/BPI_Gun.Shoot` _currentweapon))
    (:`Is Not Valid`
      (`KismetSystemLibrary.PrintString` "Cannot shoot empty gun"))))

(event `/Game/Blueprints/Interfaces/BPI_Player.Stop Sprinting`
  (set `CharacterMovementComponent.MaxWalkSpeed` 600.0 (`self.CharacterMovement`)))

(event `/Game/Blueprints/Interfaces/BPI_Player.Start Sprinting`
  (set `CharacterMovementComponent.MaxWalkSpeed` 1200.0 (`self.CharacterMovement`)))

(event `/Game/Blueprints/Interfaces/BPI_Player.Update Player Recongition`
  (params (`Is In Danger` :type Boolean))
  (set `self.IsPlayerAtRisk` `Is In Danger`))

(event `self.ReceiveTick`
  (params (DeltaSeconds :type "Float (single-precision)"))
  (bind _returnvalue (/ DeltaSeconds 10.0))
  (`self.OnRiskChange`)
  (if (`self.IsPlayerAtRisk`)
    (bind _output_get (set `self.Risk` (`KismetMathLibrary.FClamp` (+ (`self.Risk`) _returnvalue))))
    (if (>= _output_get 1.0)
      (bind _asbp_game_mode (cast `/Game/Blueprints/BP_GameMode` (`GameplayStatics.GetGameMode`)))
      (`/Game/Blueprints/BP_GameMode.Game Over (Failed)` _asbp_game_mode))
    (else
      (set `self.Risk` (`KismetMathLibrary.FClamp` (- (`self.Risk`) _returnvalue))))))

(fn `GetEquippedWeapon`
  (returns (Color :type "/Game/Blueprints/E_TargetGunColor Enum") (Type :type "/Game/Blueprints/E_WeaponType Enum") (Weapon :type "/Game/Blueprints/Weapons/BP_WeaponBase Object Reference"))
  (bind _currentweapon (`self.CurrentWeapon`))
  (if (`KismetSystemLibrary.IsValid` _currentweapon)
    (return (`/Game/Blueprints/Weapons/BP_WeaponBase.Color` _currentweapon) (`/Game/Blueprints/Weapons/BP_WeaponBase.Weapon Type` _currentweapon) _currentweapon)
    (else
      (return "NewEnumerator9" "NewEnumerator0" null))))

(fn `Hit`
  (params (`Bullet Color` :type "/Game/Blueprints/E_TargetGunColor Enum" :default "NewEnumerator9")))

(fn `UnequipCurrentWeapon`
  (returns (`Previously Equipped Weapon` :type "/Game/Blueprints/Weapons/BP_WeaponBase Object Reference"))
  (locals (PreviouslyEquipped :type "/Game/Blueprints/Weapons/BP_WeaponBase Object Reference"))
  (bind _currentweapon (`self.CurrentWeapon`))
  (`/Engine/EditorBlueprintResources/StandardMacros.IsValid` (`self.CurrentWeapon`)
    (:`Is Valid`
      (`self.K2_DetachFromActor` _currentweapon "KeepWorld" "KeepWorld" "KeepRelative")
      (message `/Game/Blueprints/Interfaces/BPI_PickableWeapon.Set Weapon Physics Simulation` _currentweapon true)
      (bind _output_get (set `local.PreviouslyEquipped` _currentweapon))
      (set `self.CurrentWeapon` null)
      (return _output_get))
    (:`Is Not Valid`
      (return null))))

(fn `UserConstructionScript`)