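; Base weapon pickup Blueprint that lets the player equip it by walking into its pickup sphere.
; When the player pawn overlaps and its equipped weapon differs in color or type, the pawn unequips its current weapon, which moves to this pickup's transform, then equips this one.
; Communication with the pawn goes through equip, unequip and get-equipped messages, and a Get Weapon Type function returns a fixed enum value.
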(event `self.Pickup Sphere Collision.OnComponentBeginOverlap`
  (params (OverlappedComponent :type "PrimitiveComponent Object Reference") (OtherActor :type "Actor Object Reference") (OtherComp :type "PrimitiveComponent Object Reference") (OtherBodyIndex :type Integer) (bFromSweep :type Boolean) (SweepResult :type "HitResult Structure (by ref)"))
  (bind _returnvalue (`GameplayStatics.GetPlayerPawn` 0))
  (bind _returnvalue_2 (`GameplayStatics.GetPlayerPawn` 0))
  (bind (_color _type) (message `/Game/Blueprints/Interfaces/BPI_Player.GetEquippedWeapon` _returnvalue))
  (if (and (not (and (`|EnumEquality` _color (`self.Color`)) (`|EnumEquality` _type (`self.Weapon Type`)))) (== _returnvalue OtherActor))
    (bind _previously_equipped_weapon (message `/Game/Blueprints/Interfaces/BPI_Player.UnequipCurrentWeapon` _returnvalue_2))
    (`/Engine/EditorBlueprintResources/StandardMacros.IsValid` _previously_equipped_weapon
      (:`Is Valid`
        (`SceneComponent.K2_SetWorldTransform` (`Actor.RootComponent` _previously_equipped_weapon) (`self.GetTransform` self) false false))
      (:`Is Not Valid`
        _))
    (message `/Game/Blueprints/Interfaces/BPI_Player.EquipWeapon` _returnvalue_2 self)))

(fn `Get Weapon Type`
  (returns (Type :type "/Game/Blueprints/E_TargetGunColor Enum"))
  (return "NewEnumerator9"))

(fn `UserConstructionScript`)