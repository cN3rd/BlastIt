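; Base gun Blueprint that fires physical projectiles and can toggle physics simulation on its mesh.
; On BeginPlay it reads the BodyColor parameter through a dynamic instance of the mesh material and caches it as ActualColor.
; Shoot spawns a scaled-down BP_Bullet at the barrel pivot, passing it Color and ActualColor.
; It then launches the bullet with a forward impulse on its sphere and plays a 2D shot sound.
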(event `self.ReceiveBeginPlay`
  (bind _returnvalue (`KismetMaterialLibrary.CreateDynamicMaterialInstance` (`PrimitiveComponent.GetMaterial` (`self.Gun Mesh`) 0)))
  (bind _returnvalue_2 (`MaterialInstanceDynamic.K2_GetVectorParameterValue` _returnvalue "BodyColor"))
  (set `self.Actual Color` _returnvalue_2))

(event `/Game/Blueprints/Interfaces/BPI_PickableWeapon.Set Weapon Physics Simulation`
  (params (Enabled :type Boolean))
  (`PrimitiveComponent.SetSimulatePhysics` (`self.Gun Mesh`) Enabled))

(event `/Game/Blueprints/Interfaces/BPI_Gun.Shoot`
  (bind _returnvalue (`|SpawnActorFromClass` "/Game/Blueprints/Weapons/BP_Bullet.BP_Bullet_C" (`KismetMathLibrary.MakeTransform` (`SceneComponent.K2_GetComponentLocation` (`self.Barrel Pivot`)) (struct) (0.1 0.1 0.1)) "Undefined" "MultiplyWithRoot" null (`self.Color`) (`self.Actual Color`) null))
  (`PrimitiveComponent.AddImpulse` (`/Game/Blueprints/Weapons/BP_Bullet.Sphere` _returnvalue) (* (`SceneComponent.GetForwardVector` (`self.Barrel Pivot`)) 2000.0) "None" false)
  (`GameplayStatics.PlaySound2D` "/Game/Audio/Sources/sci-fi-weapon-shot-02-316412.sci-fi-weapon-shot-02-316412" 1.0 1.0 0.0 null null))

(fn `UserConstructionScript`)