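; BP_Weapon is a weapon Blueprint that fires physical projectiles when its Shoot event is called.
; If the weapon is not hidden, Shoot spawns a BP_Bullet at the ShootingPosition component's world transform.
; It launches the bullet with an impulse on its Sphere along ShootingPosition's right vector, then passes WeaponType to OnCreateBullet.
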(event `Shoot`
  ;[1 0 0.009549] Shoot
  (if (not (`self.bHidden`))
    (bind _returnvalue (`|SpawnActorFromClass` "/Game/Blueprints/Guns/BP_Bullet.BP_Bullet_C" (`SceneComponent.K2_GetComponentToWorld` (`self.Shooting Position`)) "Undefined" "MultiplyWithRoot" null null))
    (`PrimitiveComponent.AddImpulse` (`/Game/Blueprints/Guns/BP_Bullet.Sphere` _returnvalue) (* (`SceneComponent.GetRightVector` (`self.Shooting Position`)) 100.0) "None" false)
    (`/Game/Blueprints/Guns/BP_Bullet.OnCreateBullet` _returnvalue (`self.Weapon Type`))))

(fn `UserConstructionScript`)