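; Base enemy that patrols a list of points with random pauses and watches for the player through a spotlight vision cone.
; Each tick it fans line traces across the vision arc, rebuilding a dynamic mesh polygon, optionally shown for debugging, when hits change.
; That hit-to-vertex conversion also detects BPI_Player actors, updates the player's recognition message, and either stops to face the player or resumes patrol.
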(event `self.ReceiveBeginPlay`
  (set `self.MovementState` "NewEnumerator1")
  (`self.MoveToNextPatrol`))

(event `OnGettingToTargte`
  ;[1 0.7959 0.2118] Patrol
  (bind _result (`/Engine/EditorBlueprintResources/StandardMacros.IncrementInt` (`self.CurrentPatrolIndex`))
    (:`  `
      (bind _output_get (set `self.CurrentPatrolIndex` _result))
      (if (> _output_get (`KismetArrayLibrary.Array_Length` (`self.PatrolPoints`)))
        (set `self.CurrentPatrolIndex` 0))
      (`self.MoveToNextPatrol`))))

(event `MoveToNextPatrol`
  ;[1 0.7959 0.2118] Patrol
  (set `self.MovementState` "NewEnumerator0")
  (`|AIMoveTo` self (0.0 0.0 0.0) (`|GetArrayItem` (`self.PatrolPoints`) (`self.CurrentPatrolIndex`))
    (:`OnSuccess`
      (set `self.MovementState` "NewEnumerator1")
      (`KismetSystemLibrary.Delay` (`KismetMathLibrary.RandomFloatInRange` 2.0 4.0))
      (set `self.MovementState` "NewEnumerator0")
      (`self.OnGettingToTargte`))))

(event `self.ReceiveActorBeginOverlap`
  (params (OtherActor :type "Actor Object Reference"))
  (bind _hitresults (`self.CreateLineTraces`))
  (set `self.LastHitResults` _hitresults))

(event `self.ReceiveTick`
  (params (DeltaSeconds :type "Float (single-precision)"))
  (bind _hitresults (`self.CreateLineTraces`))
  (bind _output_get (set `self.NewHitResults` _hitresults))
  (if (not (`KismetArrayLibrary.Array_Identical` _output_get (`self.LastHitResults`)))
    (if (`self.ShowDebuggingMeshes`)
      (bind _returnvalue (`DynamicMesh.Reset` (`self.DynamicMesh`))))
    (`GeometryScriptLibrary_MeshPrimitiveFunctions.AppendTriangulatedPolygon` _returnvalue (struct) (struct) (`self.Hit Results to Vertices` (`self.NewHitResults`)) true null)
    (set `self.LastHitResults` (`self.NewHitResults`))))

(fn `CreateLineTraces`
  (returns (HitResults :type "Array of HitResult Structure"))
  (locals (LocalHitResults :type "Array of HitResult Structure"))
  (bind _returnvalue (`self.K2_GetActorLocation`))
  (for _index (range (+ (`KismetMathLibrary.FCeil` (/ (`self.VisionArc`) (`self.TestVisionArc`))) 1))
    (if (`self.ShowDebuggingMeshes`)
      (set `self.Draw Debug Type` "ForOneFrame")
      (else
        (set `self.Draw Debug Type` "None")))
    (bind _returnvalue_2 (* _index (`self.TestVisionArc`)))
    (bind _outhit (`KismetSystemLibrary.LineTraceSingle` :`Start` _returnvalue :`End` (+ _returnvalue (`KismetMathLibrary.RotateAngleAxis` (* (`self.GetActorForwardVector`) (`self.VisionLength`)) (- (`KismetMathLibrary.FClamp` _returnvalue_2 _returnvalue_2 (`self.VisionArc`)) (/ (`self.VisionArc`) 2.0)) (0.0 0.0 1.0))) :`TraceChannel` "TraceTypeQuery1" :`DrawDebugType` (`self.Draw Debug Type`)))
    (`KismetArrayLibrary.Array_Add` (`local.LocalHitResults`) _outhit))
  (return (`local.LocalHitResults`)))

(fn `Get Enemy State`
  (returns (NewParam :type "/Game/Blueprints/Enemy/E_EnemyState Enum"))
  (return (`self.MovementState`)))

(fn `Get Enemy Type`
  (returns (`Enemy Type` :type "/Game/Blueprints/Enemy/E_EnemyType Enum"))
  (return (`self.Enemy Type`)))

(fn `Hit Results to Vertices`
  (params (HitResults :type "Array of HitResult Structure"))
  (returns (Vertices2D :type "Array of Vector2D Structure"))
  (locals (LocalVector2DVectors :type "Array of Vector2D Structure") (IsPlayerInRisk :type Boolean))
  (`KismetArrayLibrary.Array_Add` (`local.LocalVector2DVectors`))
  (for _array_element HitResults
    (`KismetArrayLibrary.Array_Add` (`local.LocalVector2DVectors`) (`KismetMathLibrary.MakeVector2D` (.x (`KismetMathLibrary.InverseTransformLocation` (`self.GetTransform`) (`KismetMathLibrary.SelectVector` (`.Location` (`GameplayStatics.BreakHitResult` _array_element)) (`.TraceEnd` (`GameplayStatics.BreakHitResult` _array_element)) (`GameplayStatics.BreakHitResult` _array_element)))) (.y (`KismetMathLibrary.InverseTransformLocation` (`self.GetTransform`) (`KismetMathLibrary.SelectVector` (`.Location` (`GameplayStatics.BreakHitResult` _array_element)) (`.TraceEnd` (`GameplayStatics.BreakHitResult` _array_element)) (`GameplayStatics.BreakHitResult` _array_element))))))
    ;[1 1 1] If Any Block Actor is a Player
    (if (`KismetSystemLibrary.DoesImplementInterface` (`.HitActor` (`GameplayStatics.BreakHitResult` _array_element)) "/Game/Blueprints/Interfaces/BPI_Player.BPI_Player_C")
      (set `local.IsPlayerInRisk` true)))
  (message `/Game/Blueprints/Interfaces/BPI_Player.Update Player Recongition` (`GameplayStatics.GetPlayerPawn` 0) (`local.IsPlayerInRisk`))
  (if (`local.IsPlayerInRisk`)
    (`self.StopToFocus`)
    (else
      (`self.MoveToNextPatrol`)))
  (return (`local.LocalVector2DVectors`)))

(fn `OnRecognizingPlayer`
  (`KismetSystemLibrary.PrintString` "Found Player")
  (`self.K2_SetActorRotation` (`KismetMathLibrary.FindLookAtRotation` (`self.K2_GetActorLocation`) (`self.K2_GetActorLocation` (`GameplayStatics.GetPlayerPawn` 0))))
  (`MovementComponent.StopMovementImmediately` (`self.CharacterMovement`))
  (set `self.MovementState` "NewEnumerator1")
  (`MovementComponent.StopMovementImmediately` (`self.CharacterMovement`)))

(fn `StopToFocus`
  (`MovementComponent.StopMovementImmediately` (`self.CharacterMovement`))
  (set `self.MovementState` "NewEnumerator1")
  (`self.K2_SetActorRotation` (`KismetMathLibrary.FindLookAtRotation` (`self.K2_GetActorLocation`) (`self.K2_GetActorLocation` (`GameplayStatics.GetPlayerPawn` 0)))))

(fn `UserConstructionScript`
  (`LocalLightComponent.SetAttenuationRadius` (`self.SpotLight`) (`self.VisionLength`))
  ;[1 1 1] Set The Angle of the Flashlight Cone
  (`SpotLightComponent.SetOuterConeAngle` (`self.SpotLight`) (/ (`self.VisionArc`) 2.0))
  (`|ExecutionSequence`
    (:`then_0`
      (if (`self.ShowDebuggingMeshes`)
        ;[1 1 1] Set the Dynamic Mesh
        (bind _returnvalue (`AddComponent|NODE_AddDynamicMeshComponent-0`))
        (bind _output_get (set `self.DynamicMeshComponent` _returnvalue))
        (bind _returnvalue_2 (`BaseDynamicMeshComponent.GetDynamicMesh` _output_get))
        (set `self.DynamicMesh` _returnvalue_2)
        (else
          (set `self.DynamicMesh` null)
          (set `self.DynamicMeshComponent` null))))
    (:`then_1`
      ;[1 1 1] Create Line Traces
      (bind _hitresults (`self.CreateLineTraces`))
      (`GeometryScriptLibrary_MeshPrimitiveFunctions.AppendTriangulatedPolygon` (`self.DynamicMesh`) (struct) (struct) (`self.Hit Results to Vertices` _hitresults) true null)
      (if (`self.ShowDebuggingMeshes`)
        (`PrimitiveComponent.SetMaterial` (`self.DynamicMeshComponent`) 0 null)))))