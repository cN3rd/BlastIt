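; BP_BaseTarget is a color-coded shootable target with a static mesh and spot light.
; The construction script creates a dynamic material instance from the mesh's first material.
; Hit compares the bullet color to the target's Color; on a match it dims the material intensity, enables physics, fires the OnTargetHit dispatcher, marks the target dead and zeroes the light's source length.
; Mismatched bullets only print a debug message.
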(fn `Hit`
  (params (`Bullet Color` :type "/Game/Blueprints/E_TargetGunColor Enum" :default "NewEnumerator9"))
  (if (`|EnumEquality` `Bullet Color` (`self.Color`))
    (`MaterialInstanceDynamic.SetScalarParameterValue` (`self.Material`) "Intensity" 0.1)
    (`PrimitiveComponent.SetSimulatePhysics` (`self.StaticMesh`) true)
    (`self.OnTargetHit`)
    (set `self.IsAlive` false)
    (`PointLightComponent.SetSourceLength` (`self.SpotLight`) 0.0)
    (return)
    (else
      (`KismetSystemLibrary.PrintString` "Ignored bullet"))))

(fn `UserConstructionScript`
  (bind _staticmesh (`self.StaticMesh`))
  (bind _returnvalue (`PrimitiveComponent.CreateDynamicMaterialInstance` _staticmesh 0 (`PrimitiveComponent.GetMaterial` _staticmesh 0) "None"))
  (set `self.Material` _returnvalue))