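; Trigger Blueprint that slides a linked door when hit, extending the parent class's OnHit.
; On BeginPlay it copies the Color parameter from the Target's mesh material to a dynamic material on its Marker.
; A hit saves the door's location and plays SlideTimeline, moving the door along negative world X by a distance scaled to its X scale.
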(event `self.ReceiveBeginPlay`
  (`parent.ReceiveBeginPlay`)
  (bind _returnvalue (`PrimitiveComponent.CreateDynamicMaterialInstance` (`self.Marker`) 0 (`PrimitiveComponent.GetMaterial` (`self.Marker`) 0) "None"))
  (bind _returnvalue_2 (`PrimitiveComponent.CreateDynamicMaterialInstance` (`/Game/Blueprints/Targets/BP_BaseTarget.StaticMesh` (`self.Target`)) 0 null "None"))
  (bind _returnvalue_3 (`MaterialInstanceDynamic.K2_GetVectorParameterValue` _returnvalue_2 "Color"))
  (`MaterialInstanceDynamic.SetVectorParameterValue` _returnvalue "Color" _returnvalue_3))

(event `Slide Door`
  (set `self.BaseDoorLocation` (`SceneComponent.K2_GetComponentLocation` (`self.Door`)))
  (bind (_direction _progress) (`Timeline|Slide Timeline`)
    (:`Update`
      ;[1 1 1] Door Sliding
      (`SceneComponent.K2_SetWorldLocation` (`self.Door`) (- (`self.BaseDoorLocation`) (`KismetMathLibrary.MakeVector` (* (.x (.scale (`SceneComponent.K2_GetComponentToWorld` (`self.Door`)))) _progress 100.0))) false false))))

(fn `OnHit`
  (`parent.OnHit`)
  (`self.Slide Door`))

(fn `UserConstructionScript`
  (`parent.UserConstructionScript`))